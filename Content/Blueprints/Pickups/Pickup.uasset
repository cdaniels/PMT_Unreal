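; Pickup actor that the player collects with the Pick input, adding its ItemType to the item count on MyGameMode_BP.
; A trigger overlap with MyFPCharacter enables pickup and shows a PickupPrompt widget, both cleared when the overlap ends.
; On pickup it finds MyGameMode_BP via GetActorOfClass, reports the item, plays an explosion sound and particle effect, then destroys itself.
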(event `InputAction|Pick` :consume false
  (params (Key :type "Key Structure"))
  (:`Pressed`
    (if (`self.IsPickupable`)
      (bind _returnvalue (`GameplayStatics.GetActorOfClass` "/Game/Blueprints/MyGameMode_BP.MyGameMode_BP_C"))
      (`/Game/Blueprints/MyGameMode_BP.AddItemCount` _returnvalue (`self.ItemType`))
      (`self.PickupPlaySound`))))

(event `PickupPlaySound`
  (`GameplayStatics.SpawnSoundAtLocation` "/Game/StarterContent/Audio/Explosion01.Explosion01" (`self.K2_GetActorLocation`) (struct) 1.0 1.0 0.0 null null)
  (`GameplayStatics.SpawnEmitterAtLocation` "/Game/StarterContent/Particles/P_Explosion.P_Explosion" (`self.K2_GetActorLocation`))
  (`self.K2_DestroyActor`))

(event `self.Trigger.OnComponentBeginOverlap`
  (params (OverlappedComponent :type "PrimitiveComponent Object Reference") (OtherActor :type "Actor Object Reference") (OtherComp :type "PrimitiveComponent Object Reference") (OtherBodyIndex :type Integer) (bFromSweep :type Boolean) (SweepResult :type "HitResult Structure (by ref)"))
  (cast `/Game/Blueprints/MyFPCharacter` OtherActor)
  (set `self.IsPickupable` true)
  (bind _returnvalue (`|CreateWidget` "/Game/Blueprints/HUD/PickupPrompt.PickupPrompt_C"))
  (`UserWidget.AddToViewport` _returnvalue 0))

(event `self.Trigger.OnComponentEndOverlap`
  (params (OverlappedComponent :type "PrimitiveComponent Object Reference") (OtherActor :type "Actor Object Reference") (OtherComp :type "PrimitiveComponent Object Reference") (OtherBodyIndex :type Integer))
  (cast `/Game/Blueprints/MyFPCharacter` OtherActor)
  (set `self.IsPickupable` false)
  (`Widget.RemoveFromParent` (stale `self.Trigger.OnComponentBeginOverlap` _returnvalue)))

(fn `UserConstructionScript`)