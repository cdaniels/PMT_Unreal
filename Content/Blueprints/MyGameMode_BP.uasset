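; Game mode that runs a timed round, tallies collected fire extinguishers, fires and life potions, and scores them.
; BeginPlay shows the item count widget, and Tick uses a one-second Delay to drive the minutes/seconds countdown.
; At zero it computes player score from potions and team score from extinguishers minus fires and potions, then shows RoundOver and pauses.
; Robot team scoring and player count reset are defined but not called here.
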(event `self.ReceiveBeginPlay`
  (bind _returnvalue (`|CreateWidget` "/Game/Blueprints/HUD/ItemCount.ItemCount_C"))
  (`UserWidget.AddToViewport` _returnvalue 0))

(event `self.ReceiveTick`
  (params (DeltaSeconds :type "Float (single-precision)"))
  (`KismetSystemLibrary.Delay` 1.0)
  (if (== (`self.Seconds`) 0)
    (if (== (`self.Minutes`) 0)
      (`self.UpdatePlayerScore`)
      (`self.UpdateTeamScore_ForPlayer`)
      (bind _returnvalue (`|CreateWidget` "/Game/Blueprints/HUD/RoundOver.RoundOver_C"))
      (`UserWidget.AddToViewport` _returnvalue 0)
      (set `PlayerController.bShowMouseCursor` true (`GameplayStatics.GetPlayerController` 0))
      (`GameplayStatics.SetGamePaused` true)
      (else
        (set `self.Seconds` 59)
        (set `self.Minutes` (- (`self.Minutes`) 1))))
    (else
      (set `self.Seconds` (- (`self.Seconds`) 1)))))

(fn `AddItemCount`
  (params (ItemType :type "/Game/Blueprints/Pickups/PickupableItems Enum" :default "NewEnumerator0"))
  (switch `/Game/Blueprints/Pickups/PickupableItems` ItemType
    (:`NewEnumerator0`
      (set `self.Player_ExtinguisherCount_Int` (+ (`self.Player_ExtinguisherCount_Int`) 1)))
    (:`NewEnumerator1`
      (set `self.Player_FireCount_Int` (+ (`self.Player_FireCount_Int`) 1)))
    (:`NewEnumerator2`
      (set `self.Player_LifePotionCount_Int` (+ (`self.Player_LifePotionCount_Int`) 1)))))

(fn `ResetPlayerItemCount`
  (set `self.Player_FireCount_Int` 0)
  (set `self.Player_ExtinguisherCount_Int` 0)
  (set `self.Player_LifePotionCount_Int` 0))

(fn `UpdatePlayerScore`
  (set `self.Player_Score_Int` (* (`self.Player_LifePotionCount_Int`) 100)))

(fn `UpdateTeamScore_ForPlayer`
  (set `self.Team_Score_Int` (- (* (`self.Player_ExtinguisherCount_Int`) 100) (+ (* (`self.Player_FireCount_Int`) 100) (* (`self.Player_LifePotionCount_Int`) 100)))))

(fn `UpdateTeamScore_ForRobot`
  (set `self.Team_Score_Int` (- (* (`self.Robot_ExtinguisherCount_Int`) 100) (+ (* (`self.Robot_FireCount_Int`) 100) (* (`self.Robot_LifePotionCount_Int`) 100)))))

(fn `UserConstructionScript`)